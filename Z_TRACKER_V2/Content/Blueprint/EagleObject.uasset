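; EagleObject is a rotation puzzle Blueprint that checks whether an actor sits at a target orientation.
; A looping half-second timer from BeginPlay runs CHECK PUZZLE, which tests roll, pitch and yaw against narrow tolerance ranges.
; A match sets IsSolved and adds a new widget to the viewport on every passing check, as the timer is never cleared.
; Failed checks also set IsSolved to true.
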(event EventBeginPlay
  (Utilities|Time|SetTimerbyFunctionName 0 "CHECK PUZZLE" 0.5 true))

(event Collision|EventActorBeginOverlap
  (params (OtherActor :type Actor%20Object%20Reference)))

(event EventTick
  (params (DeltaSeconds :type Float%20%28single-precision%29)))

(fn ConstructionScript)

(fn CHECKPUZZLE
  (bind _actor (Variables|Components|GetActor))
  (bind _returnvalue (Transformation|GetActorRotation _actor))
  (if (Math|Float|InRange(Float) (.roll _returnvalue) 85.0 95.0)
    (if (Math|Float|InRange(Float) (.pitch _returnvalue) -5.0 5.0)
      (if (Math|Float|InRange(Float) (.yaw _returnvalue) 85.0 95.0)
        (Variables|Default|SetIsSolved true)
        (bind _returnvalue_2 (UserInterface|CreateWidget "/Game/ui.ui_C"))
        (bind _output_get (Variables|Default|SetNewVar_0 _returnvalue_2))
        (UserInterface|Viewport|AddtoViewport _output_get 0)
        (else
          (Variables|Default|SetIsSolved true :!label _label)))
      (else
        (goto _label)))
    (else
      (goto _label))))