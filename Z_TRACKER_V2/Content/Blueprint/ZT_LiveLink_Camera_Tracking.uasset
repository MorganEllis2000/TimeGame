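; Live Link camera tracking template actor that drives a target actor's rotation from streamed orientation data, using placeholder actor and camera references.
; On each Live Link update, it applies the Basic role's first four properties as its own quaternion rotation.
; The negated rotation passes through a weighted moving average to the target, then the view switches to the camera and the value prints on screen.
; A quantizing Smooth function is defined but not called.
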(event OnLiveLinkUpdated(LiveLinkComponentController)
  (params (DeltaTime :type Float%20%28single-precision%29))
  (bind _self self)
  (bind _returnvalue (Transformation|GetActorTransform _self))
  (bind _dataresult (|EvaluateLiveLinkFramewithSpecificRole "(Name=\"Z_Tracker01\")" "/Script/LiveLinkInterface.LiveLinkBasicRole") ; Delete and replace this node once LiveLink is connected
    (:then
      (Variables|Default|SetpropertyValues (.PropertyValues (Utilities|Struct|BreakLiveLinkBaseFrameData (.FrameData (Utilities|Struct|BreakLiveLinkBasicBlueprintData _dataresult)))))
      (Class|ZTQuaternionRotationBPLibrary|SetActorRelativeRotationQuat _self (Utilities|Struct|MakeQuat (Utilities|Array|Get(acopy) (Variables|Default|GetpropertyValues)) (Utilities|Array|Get(acopy) (Variables|Default|GetpropertyValues) 1) (Utilities|Array|Get(acopy) (Variables|Default|GetpropertyValues) 2) (Utilities|Array|Get(acopy) (Variables|Default|GetpropertyValues) 3)))
      (Transformation|SetActorRelativeRotation (Variables|Default|Getyour_actor_here) (Class|KismetMathLibrary|WeightedMovingAverageFRotator (Math|Rotator|MakeRotator (* (.roll (.rotation _returnvalue)) -1.0) (* (.pitch (.rotation _returnvalue)) -1.0) (* (.yaw (.rotation _returnvalue)) -1.0)) (Variables|Default|GetPreRot) 0.5))
      (Variables|Default|SetPreRot (Class|KismetMathLibrary|WeightedMovingAverageFRotator (Math|Rotator|MakeRotator (* (.roll (.rotation _returnvalue)) -1.0) (* (.pitch (.rotation _returnvalue)) -1.0) (* (.yaw (.rotation _returnvalue)) -1.0)) (Variables|Default|GetPreRot) 0.5))
      (Game|Player|SetViewTargetwithBlend (Game|GetPlayerController 0) (Variables|Default|Getyour_camera_here) 0.0 "VTBlend_Linear" 0.0 false)
      (Development|PrintString (Utilities|String|ToString(Rotator) (Class|KismetMathLibrary|WeightedMovingAverageFRotator (Math|Rotator|MakeRotator (* (.roll (.rotation _returnvalue)) -1.0) (* (.pitch (.rotation _returnvalue)) -1.0) (* (.yaw (.rotation _returnvalue)) -1.0)) (Variables|Default|GetPreRot) 0.5)) true false "(R=1.000000,G=0.180784,B=0.844464,A=1.000000)" 0.2))))

(event EventBeginPlay)

(event Collision|EventActorBeginOverlap
  (params (OtherActor :type Actor%20Object%20Reference)))

(fn ConstructionScript)

(fn Smooth
  (params (Rotation_In :type Rotator) (smoothness :type Float%20%28single-precision%29))
  (bind _returnvalue (* smoothness (.yaw Rotation_In)))
  (bind _returnvalue_2 (* smoothness (.pitch Rotation_In)))
  (bind _returnvalue_3 (* smoothness (.roll Rotation_In)))
  (return (Math|Rotator|MakeRotator (/ (Math|Conversions|ToFloat(Integer) (/ (+ (Math|Float|Round _returnvalue_3) (Math|Float|Truncate _returnvalue_3)) 2)) smoothness) (/ (Math|Conversions|ToFloat(Integer) (/ (+ (Math|Float|Round _returnvalue_2) (Math|Float|Truncate _returnvalue_2)) 2)) smoothness) (/ (Math|Conversions|ToFloat(Integer) (/ (+ (Math|Float|Round _returnvalue) (Math|Float|Truncate _returnvalue)) 2)) smoothness))))